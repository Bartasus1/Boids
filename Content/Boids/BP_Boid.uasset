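; BP_Boid is a boid actor Blueprint with events for bounds handling and movement-facing rotation.
; Edges compares the absolute world location against the supplied Bounds and, when any axis reaches its limit, teleports the actor without sweep to its location multiplied by -2, across the origin.
; RotateToMovement aligns the actor's X axis with its Velocity, which nothing in this graph updates.
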(event `Edges`
  (params (Bounds :type "Vector Structure"))
  (bind _returnvalue (`self.K2_GetActorLocation`))
  (bind (_returnvalue_x _returnvalue_y _returnvalue_z) (`KismetMathLibrary.BreakVector` (`KismetMathLibrary.Vector_GetAbs` _returnvalue)))
  (if (or (<= Bounds_X _returnvalue_x) (<= Bounds_Y _returnvalue_y) (<= Bounds_Z _returnvalue_z))
    (`self.K2_SetActorLocation` (* _returnvalue -2.0) false true)))

(event `RotateToMovement`
  (`self.K2_SetActorRotation` (`KismetMathLibrary.MakeRotFromX` (`self.Velocity`))))

(fn `UserConstructionScript`)